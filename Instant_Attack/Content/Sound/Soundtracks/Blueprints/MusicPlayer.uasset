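; Music player actor that plays random background soundtracks continuously during the game.
; On BeginPlay, AddSoundtracks spawns a GameSoundtrack actor for each hard-coded cue and duration into an array, then a random one starts.
; An endless DelayedLoop macro calls CheckMusic every second, counting elapsed time against the current track's stored duration rather than detecting audio completion.
; When time runs out, it picks another random track, possibly the same one.
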(event EventBeginPlay
  (bind _soundtracks (Variables|Default|GetSoundtracks))
  (CallFunction|AddSoundtracks)
  (bind _output_get (Variables|Default|SetCurrentSoundtrack (Utilities|Array|Get(acopy) _soundtracks (Math|Random|RandomIntegerinRange 0 (- (Utilities|Array|Length _soundtracks) 1)))))
  (Default|PlaySoundtrack _output_get)
  (Utilities|DelayedLoop false 1.0
    (:LoopBody
      (CallFunction|CheckMusic))))

(event Collision|EventActorBeginOverlap
  (params (OtherActor :type Actor%20Object%20Reference)))

(event EventTick
  (params (DeltaSeconds :type Float%20%28single-precision%29)))

(fn ConstructionScript)

(fn AddSoundtracks
  (bind _returnvalue (Game|SpawnActorfromClass "/Game/Sound/Soundtracks/Blueprints/GameSoundtrack.GameSoundtrack_C" (Variables|Default|GetSoundtrackSpawnTransform) "Undefined" 0 116.0 "/Game/Sound/Soundtracks/Assets/57th_expedition_Cue.57th_expedition_Cue"))
  (Utilities|Array|Add (Variables|Default|GetSoundtracks) _returnvalue)
  (bind _returnvalue_2 (Game|SpawnActorfromClass "/Game/Sound/Soundtracks/Blueprints/GameSoundtrack.GameSoundtrack_C" (Variables|Default|GetSoundtrackSpawnTransform) "Undefined" 0 3.6e+02 "/Game/Sound/Soundtracks/Assets/Achilles_leads_the_myrmidons_Cue.Achilles_leads_the_myrmidons_Cue"))
  (Utilities|Array|Add (Variables|Default|GetSoundtracks) _returnvalue_2)
  (bind _returnvalue_3 (Game|SpawnActorfromClass "/Game/Sound/Soundtracks/Blueprints/GameSoundtrack.GameSoundtrack_C" (Variables|Default|GetSoundtrackSpawnTransform) "Undefined" 0 2.3e+02 "/Game/Sound/Soundtracks/Assets/Anakin_s_betrayal_Cue.Anakin_s_betrayal_Cue"))
  (Utilities|Array|Add (Variables|Default|GetSoundtracks) _returnvalue_3)
  (bind _returnvalue_4 (Game|SpawnActorfromClass "/Game/Sound/Soundtracks/Blueprints/GameSoundtrack.GameSoundtrack_C" (Variables|Default|GetSoundtrackSpawnTransform) "Undefined" 0 1.2e+02 "/Game/Sound/Soundtracks/Assets/Arrival_Cue.Arrival_Cue"))
  (Utilities|Array|Add (Variables|Default|GetSoundtracks) _returnvalue_4)
  (bind _returnvalue_5 (Game|SpawnActorfromClass "/Game/Sound/Soundtracks/Blueprints/GameSoundtrack.GameSoundtrack_C" (Variables|Default|GetSoundtrackSpawnTransform) "Undefined" 0 286.0 "/Game/Sound/Soundtracks/Assets/At_wit_s_end_Cue.At_wit_s_end_Cue"))
  (Utilities|Array|Add (Variables|Default|GetSoundtracks) _returnvalue_5)
  (bind _returnvalue_6 (Game|SpawnActorfromClass "/Game/Sound/Soundtracks/Blueprints/GameSoundtrack.GameSoundtrack_C" (Variables|Default|GetSoundtrackSpawnTransform) "Undefined" 0 163.0 "/Game/Sound/Soundtracks/Assets/Battle_Cue.Battle_Cue"))
  (Utilities|Array|Add (Variables|Default|GetSoundtracks) _returnvalue_6)
  (bind _returnvalue_7 (Game|SpawnActorfromClass "/Game/Sound/Soundtracks/Blueprints/GameSoundtrack.GameSoundtrack_C" (Variables|Default|GetSoundtrackSpawnTransform) "Undefined" 0 164.0 "/Game/Sound/Soundtracks/Assets/Champions_League_Cue.Champions_League_Cue"))
  (Utilities|Array|Add (Variables|Default|GetSoundtracks) _returnvalue_7)
  (bind _returnvalue_8 (Game|SpawnActorfromClass "/Game/Sound/Soundtracks/Blueprints/GameSoundtrack.GameSoundtrack_C" (Variables|Default|GetSoundtrackSpawnTransform) "Undefined" 0 68.0 "/Game/Sound/Soundtracks/Assets/Cookies_Cue.Cookies_Cue"))
  (Utilities|Array|Add (Variables|Default|GetSoundtracks) _returnvalue_8)
  (bind _returnvalue_9 (Game|SpawnActorfromClass "/Game/Sound/Soundtracks/Blueprints/GameSoundtrack.GameSoundtrack_C" (Variables|Default|GetSoundtrackSpawnTransform) "Undefined" 0 102.0 "/Game/Sound/Soundtracks/Assets/Do_what_you_were_made_for_Cue.Do_what_you_were_made_for_Cue"))
  (Utilities|Array|Add (Variables|Default|GetSoundtracks) _returnvalue_9)
  (bind _returnvalue_10 (Game|SpawnActorfromClass "/Game/Sound/Soundtracks/Blueprints/GameSoundtrack.GameSoundtrack_C" (Variables|Default|GetSoundtrackSpawnTransform) "Undefined" 0 196.0 "/Game/Sound/Soundtracks/Assets/FirstClass_Cue.FirstClass_Cue"))
  (Utilities|Array|Add (Variables|Default|GetSoundtracks) _returnvalue_10)
  (bind _returnvalue_11 (Game|SpawnActorfromClass "/Game/Sound/Soundtracks/Blueprints/GameSoundtrack.GameSoundtrack_C" (Variables|Default|GetSoundtrackSpawnTransform) "Undefined" 0 73.0 "/Game/Sound/Soundtracks/Assets/For_Old_Time_s_sake_Cue.For_Old_Time_s_sake_Cue"))
  (Utilities|Array|Add (Variables|Default|GetSoundtracks) _returnvalue_11)
  (bind _returnvalue_12 (Game|SpawnActorfromClass "/Game/Sound/Soundtracks/Blueprints/GameSoundtrack.GameSoundtrack_C" (Variables|Default|GetSoundtrackSpawnTransform) "Undefined" 0 112.0 "/Game/Sound/Soundtracks/Assets/Heat_Cue.Heat_Cue"))
  (Utilities|Array|Add (Variables|Default|GetSoundtracks) _returnvalue_12)
  (bind _returnvalue_13 (Game|SpawnActorfromClass "/Game/Sound/Soundtracks/Blueprints/GameSoundtrack.GameSoundtrack_C" (Variables|Default|GetSoundtrackSpawnTransform) "Undefined" 0 183.0 "/Game/Sound/Soundtracks/Assets/Imperial_Guard_Cue.Imperial_Guard_Cue"))
  (Utilities|Array|Add (Variables|Default|GetSoundtracks) _returnvalue_13)
  (bind _returnvalue_14 (Game|SpawnActorfromClass "/Game/Sound/Soundtracks/Blueprints/GameSoundtrack.GameSoundtrack_C" (Variables|Default|GetSoundtrackSpawnTransform) "Undefined" 0 214.0 "/Game/Sound/Soundtracks/Assets/Martha_Cue.Martha_Cue"))
  (Utilities|Array|Add (Variables|Default|GetSoundtracks) _returnvalue_14)
  (bind _returnvalue_15 (Game|SpawnActorfromClass "/Game/Sound/Soundtracks/Blueprints/GameSoundtrack.GameSoundtrack_C" (Variables|Default|GetSoundtrackSpawnTransform) "Undefined" 0 1.8e+02 "/Game/Sound/Soundtracks/Assets/My_Brother_Cue.My_Brother_Cue"))
  (Utilities|Array|Add (Variables|Default|GetSoundtracks) _returnvalue_15)
  (bind _returnvalue_16 (Game|SpawnActorfromClass "/Game/Sound/Soundtracks/Blueprints/GameSoundtrack.GameSoundtrack_C" (Variables|Default|GetSoundtrackSpawnTransform) "Undefined" 0 176.0 "/Game/Sound/Soundtracks/Assets/Open_your_friend_s_eyes_Cue.Open_your_friend_s_eyes_Cue"))
  (Utilities|Array|Add (Variables|Default|GetSoundtracks) _returnvalue_16)
  (bind _returnvalue_17 (Game|SpawnActorfromClass "/Game/Sound/Soundtracks/Blueprints/GameSoundtrack.GameSoundtrack_C" (Variables|Default|GetSoundtrackSpawnTransform) "Undefined" 0 324.0 "/Game/Sound/Soundtracks/Assets/Pruit_Igoe_and_prophecies_Cue.Pruit_Igoe_and_prophecies_Cue"))
  (Utilities|Array|Add (Variables|Default|GetSoundtracks) _returnvalue_17)
  (bind _returnvalue_18 (Game|SpawnActorfromClass "/Game/Sound/Soundtracks/Blueprints/GameSoundtrack.GameSoundtrack_C" (Variables|Default|GetSoundtrackSpawnTransform) "Undefined" 0 2.8e+02 "/Game/Sound/Soundtracks/Assets/Sarabande_Cue.Sarabande_Cue"))
  (Utilities|Array|Add (Variables|Default|GetSoundtracks) _returnvalue_18)
  (bind _returnvalue_19 (Game|SpawnActorfromClass "/Game/Sound/Soundtracks/Blueprints/GameSoundtrack.GameSoundtrack_C" (Variables|Default|GetSoundtrackSpawnTransform) "Undefined" 0 206.0 "/Game/Sound/Soundtracks/Assets/SpaceMarines_Cue.SpaceMarines_Cue"))
  (Utilities|Array|Add (Variables|Default|GetSoundtracks) _returnvalue_19)
  (bind _returnvalue_20 (Game|SpawnActorfromClass "/Game/Sound/Soundtracks/Blueprints/GameSoundtrack.GameSoundtrack_C" (Variables|Default|GetSoundtrackSpawnTransform) "Undefined" 0 73.0 "/Game/Sound/Soundtracks/Assets/SubLift_Cue.SubLift_Cue"))
  (Utilities|Array|Add (Variables|Default|GetSoundtracks) _returnvalue_20)
  (bind _returnvalue_21 (Game|SpawnActorfromClass "/Game/Sound/Soundtracks/Blueprints/GameSoundtrack.GameSoundtrack_C" (Variables|Default|GetSoundtrackSpawnTransform) "Undefined" 0 135.0 "/Game/Sound/Soundtracks/Assets/The_dark_world_Cue.The_dark_world_Cue"))
  (Utilities|Array|Add (Variables|Default|GetSoundtracks) _returnvalue_21)
  (bind _returnvalue_22 (Game|SpawnActorfromClass "/Game/Sound/Soundtracks/Blueprints/GameSoundtrack.GameSoundtrack_C" (Variables|Default|GetSoundtrackSpawnTransform) "Undefined" 0 97.0 "/Game/Sound/Soundtracks/Assets/TheDarkKnightRises_Cue.TheDarkKnightRises_Cue"))
  (Utilities|Array|Add (Variables|Default|GetSoundtracks) _returnvalue_22)
  (bind _returnvalue_23 (Game|SpawnActorfromClass "/Game/Sound/Soundtracks/Blueprints/GameSoundtrack.GameSoundtrack_C" (Variables|Default|GetSoundtrackSpawnTransform) "Undefined" 0 237.0 "/Game/Sound/Soundtracks/Assets/Vogel_Cue.Vogel_Cue"))
  (Utilities|Array|Add (Variables|Default|GetSoundtracks) _returnvalue_23)
  (bind _returnvalue_24 (Game|SpawnActorfromClass "/Game/Sound/Soundtracks/Blueprints/GameSoundtrack.GameSoundtrack_C" (Variables|Default|GetSoundtrackSpawnTransform) "Undefined" 0 168.0 "/Game/Sound/Soundtracks/Assets/What_is_necessary_Cue.What_is_necessary_Cue"))
  (Utilities|Array|Add (Variables|Default|GetSoundtracks) _returnvalue_24)
  (bind _returnvalue_25 (Game|SpawnActorfromClass "/Game/Sound/Soundtracks/Blueprints/GameSoundtrack.GameSoundtrack_C" (Variables|Default|GetSoundtrackSpawnTransform) "Undefined" 0 207.0 "/Game/Sound/Soundtracks/Assets/You_re_a_soldier_now_Cue.You_re_a_soldier_now_Cue"))
  (Utilities|Array|Add (Variables|Default|GetSoundtracks) _returnvalue_25))

(fn CheckMusic
  (bind _soundtracks (Variables|Default|GetSoundtracks))
  (if (> (Variables|Default|GetTimeSpent) (Variables|/Game/Sound/Soundtracks/Blueprints/GameSoundtrack.GameSoundtrack_C|GetSoundtrackTime (Variables|Default|GetCurrentSoundtrack)))
    (Variables|Default|SetTimeSpent 0.0)
    (bind _output_get (Variables|Default|SetCurrentSoundtrack (Utilities|Array|Get(acopy) _soundtracks (Math|Random|RandomIntegerinRange 0 (- (Utilities|Array|Length _soundtracks) 1)))))
    (Default|PlaySoundtrack _output_get)
    (else
      (Math|Float|IncrementFloat (Variables|Default|GetTimeSpent)))))